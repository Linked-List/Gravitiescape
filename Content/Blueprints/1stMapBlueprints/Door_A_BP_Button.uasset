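; Door Blueprint for the first map that slides open when something enters its trigger, gated by two puzzle conditions.
; On overlap it checks that the laptop Blueprint reports IsManipulated and the emergency button Blueprint reports DoorOpened, fetching both with GetActorOfClass.
; If both hold, it activates two steam effects and plays a Timeline that lerps the door mesh between closed and open locations.
; Leaving the trigger reverses the Timeline to close it.
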(event OnComponentBeginOverlap(Trigger)
  (params (OverlappedComponent :type Primitive%20Component%20Object%20Reference) (OtherActor :type Actor%20Object%20Reference) (OtherComp :type Primitive%20Component%20Object%20Reference) (OtherBodyIndex :type Integer) (bFromSweep :type Boolean) (SweepResult :type Hit%20Result%20Structure%20%28by%20ref%29))
  ;[1 1 1] Gravity Manipulation Detection
  (bind _returnvalue (Actor|GetActorOfClass "/Game/Blueprints/1stMapBlueprints/SM_Laptop_BP.SM_Laptop_BP_C"))
  (if (Variables|/Game/Blueprints/1stMapBlueprints/SM_Laptop_BP.SM_Laptop_BP_C|GetisManipulated _returnvalue)
    ;[1 1 1] Button Click Detection
    (bind _returnvalue_2 (Actor|GetActorOfClass "/Game/Blueprints/1stMapBlueprints/SM_EmergencyButton_Blueprint2.SM_EmergencyButton_Blueprint2_C"))
    (if (Variables|/Game/Blueprints/1stMapBlueprints/SM_EmergencyButton_Blueprint2.SM_EmergencyButton_Blueprint2_C|GetdoorOpened _returnvalue_2)
      ;[1 1 1] Door Open & Close
      (Components|Activation|Activate (Variables|Default|GetSteamDoor) false)
      (bind _doorposition (Timeline|Timeline_0 Play)
        (:Update
          (Transformation|SetRelativeLocation (Variables|Default|GetDoor_Small_A) (Math|Vector|Lerp(Vector) (Variables|Door|GetDoorClosed) (Variables|Door|GetDoorOpen) _doorposition) false false))))))

(event OnComponentEndOverlap(Trigger)
  (params (OverlappedComponent :type Primitive%20Component%20Object%20Reference) (OtherActor :type Actor%20Object%20Reference) (OtherComp :type Primitive%20Component%20Object%20Reference) (OtherBodyIndex :type Integer))
  ;[1 1 1] Door Open & Close
  (bind _doorposition (Timeline|Timeline_0 Reverse)
    (:Update
      (Transformation|SetRelativeLocation (Variables|Default|GetDoor_Small_A) (Math|Vector|Lerp(Vector) (Variables|Door|GetDoorClosed) (Variables|Door|GetDoorOpen) _doorposition) false false))))

(fn ConstructionScript)