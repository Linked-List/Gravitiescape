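; Level Sequence director Blueprint for the first stage sequence, which locks player control while it plays.
; Two event-track functions bound to CineCameraActor1 toggle the IsLoading flag on GravityGameMode and disable, then re-enable, input on player character 0.
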(event Custom|CineCameraActor1_Event_0
  (params (CineCameraActor1 :type Cine%20Camera%20Actor%20Object%20Reference))
  ;[1 1 1] Disable Inputs while Sequence
  (bind _asgravity_game_mode (Utilities|Casting|CastToGravityGameMode (Game|GetGameMode)))
  (Variables|/Game/Blueprints/GravityGameMode.GravityGameMode_C|SetisLoading _asgravity_game_mode true)
  (Input|DisableInput (Game|GetPlayerCharacter 0) (Game|GetPlayerController 0)))

(event Custom|CineCameraActor1_Event_1
  (params (CineCameraActor1 :type Cine%20Camera%20Actor%20Object%20Reference))
  ;[1 1 1] Enable Inputs after Sequence
  (bind _asgravity_game_mode (Utilities|Casting|CastToGravityGameMode (Game|GetGameMode)))
  (Variables|/Game/Blueprints/GravityGameMode.GravityGameMode_C|SetisLoading _asgravity_game_mode false)
  (Input|EnableInput (Game|GetPlayerCharacter 0) (Game|GetPlayerController 0)))