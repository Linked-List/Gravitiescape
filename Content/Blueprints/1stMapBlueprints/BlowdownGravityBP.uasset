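; Overlap actor that alters gravity for a ThirdPersonCharacter inside its bounds.
; On begin overlap it raises the character's GravityScale to triple and adds a single upward force through CharacterMovement.
; On end overlap it adds the opposite downward force and sets GravityScale back to a fixed default rather than a saved value.
; Other overlapping actors only print a cast-failure message.
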(event Collision|EventActorBeginOverlap
  (params (OtherActor :type Actor%20Object%20Reference))
  (bind _asthird_person_character (Utilities|Casting|CastToThirdPersonCharacter OtherActor)
    (:then
      ;[1 1 1] Set Gravity Scale & Add Force
      (Physics|AddForce (Variables|/Script/Engine.Character|GetCharacterMovement _asthird_person_character) "0, 0,500.000000")
      (Variables|/Script/Engine.CharacterMovementComponent|SetGravityScale (Variables|/Script/Engine.Character|GetCharacterMovement _asthird_person_character) 3.0))
    (:CastFailed
      (Development|PrintString "Cast Failed!"))))

(event Collision|EventActorEndOverlap
  (params (OtherActor :type Actor%20Object%20Reference))
  (bind _asthird_person_character (Utilities|Casting|CastToThirdPersonCharacter OtherActor)
    (:then
      ;[1 1 1] Reset Gravity Scale & Force
      (Physics|AddForce (Variables|/Script/Engine.Character|GetCharacterMovement _asthird_person_character) "0, 0,-500.000000")
      (Variables|/Script/Engine.CharacterMovementComponent|SetGravityScale (Variables|/Script/Engine.Character|GetCharacterMovement _asthird_person_character) 1.0))
    (:CastFailed
      (Development|PrintString "Cast Failed!"))))

(fn ConstructionScript)