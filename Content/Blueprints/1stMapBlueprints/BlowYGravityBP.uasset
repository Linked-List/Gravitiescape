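; Overlap actor that acts as a low-gravity blow zone, pushing the ThirdPersonCharacter along world negative Y.
; On begin overlap it halves the character's gravity scale and subtracts a fixed Y amount from its movement velocity, a one-time impulse rather than continuous force.
; On end overlap it sets gravity scale back to a hard-coded normal value; other overlapping actors only print a cast failure message.
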(event EventBeginPlay)

(event Collision|EventActorBeginOverlap
  (params (OtherActor :type Actor%20Object%20Reference))
  (bind _asthird_person_character (Utilities|Casting|CastToThirdPersonCharacter OtherActor)
    (:then
      ;[1 1 1] Set Gravity Scale
      (Variables|/Script/Engine.CharacterMovementComponent|SetGravityScale (Variables|/Script/Engine.Character|GetCharacterMovement _asthird_person_character) 0.5)
      ;[1 1 1] Set Velocity
      (Variables|/Script/Engine.MovementComponent|SetVelocity (Variables|/Script/Engine.Character|GetCharacterMovement _asthird_person_character) (- (Variables|/Script/Engine.MovementComponent|GetVelocity (Variables|/Script/Engine.Character|GetCharacterMovement _asthird_person_character)) "0,500.000000, 0")))
    (:CastFailed
      (Development|PrintString "Cast Failed!"))))

(event Collision|EventActorEndOverlap
  (params (OtherActor :type Actor%20Object%20Reference))
  (bind _asthird_person_character (Utilities|Casting|CastToThirdPersonCharacter OtherActor)
    (:then
      ;[1 1 1] Reset Gravity Scale
      (Variables|/Script/Engine.CharacterMovementComponent|SetGravityScale (Variables|/Script/Engine.Character|GetCharacterMovement _asthird_person_character) 1.0))
    (:CastFailed
      (Development|PrintString "Cast Failed!"))))

(fn ConstructionScript)