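; Door Blueprint whose small door mesh is opened and closed through custom OpenDoor and CloseDoor events, presumably driven by an external switch.
; Each event snaps the mesh's relative location instantly between the closed origin and a raised position.
; The trigger overlap events are empty, and a timeline lerp with steam effect activation is left disconnected, so it never runs.
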(event OnComponentBeginOverlap(Trigger)
  (params (OverlappedComponent :type Primitive%20Component%20Object%20Reference) (OtherActor :type Actor%20Object%20Reference) (OtherComp :type Primitive%20Component%20Object%20Reference) (OtherBodyIndex :type Integer) (bFromSweep :type Boolean) (SweepResult :type Hit%20Result%20Structure%20%28by%20ref%29)))

(event OnComponentEndOverlap(Trigger)
  (params (OverlappedComponent :type Primitive%20Component%20Object%20Reference) (OtherActor :type Actor%20Object%20Reference) (OtherComp :type Primitive%20Component%20Object%20Reference) (OtherBodyIndex :type Integer)))

(event Custom|Open%20Door
  (Transformation|SetRelativeLocation (Variables|Default|GetDoor_Small_A) "0, 0,268.000000" false false))

(event Custom|Close%20Door
  (Transformation|SetRelativeLocation (Variables|Default|GetDoor_Small_A) "0, 0, 0" false false))

(fn ConstructionScript)