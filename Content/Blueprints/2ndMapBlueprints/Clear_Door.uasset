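; Clear_Door is a door Blueprint in the second-map folder that slides open once, with steam effects.
; OpenDoor checks and sets the IsOpen flag so that DoorAction fires only on the first call.
; DoorAction activates two steam components and plays a timeline that lerps DoorSmallA's relative location from the closed to the open position.
; The file contains no closing logic.
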(event Custom|DoorAction
  (Components|Activation|Activate (Variables|Default|GetSteamDoor) false)
  (bind _doorposition (Timeline|Timeline_0 Play)
    (:Update
      (Transformation|SetRelativeLocation (Variables|Default|GetDoor_Small_A) (Math|Vector|Lerp(Vector) (Variables|Door|GetDoorClosed) (Variables|Door|GetDoorOpen) _doorposition) false false))))

(fn ConstructionScript)

(fn OpenDoor
  (if (not (Variables|Default|GetisOpen))
    (Variables|Default|SetisOpen true)
    (CallFunction|DoorAction)))