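; Directional gravity volume that pulls overlapping actors along its own rotated down axis.
; Each Tick it rotates the down vector by the actor's rotation, scales it by GravityScale and passes it to each overlapping Gravity_Object via SetCubeGravity.
; With AffectCharacter on, it also aligns each overlapping Stage2Character to its rotation, adds that vector as force and overwrites the character's velocity with it.
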(event EventTick
  (params (DeltaSeconds :type Float%20%28single-precision%29))
  (bind _returnvalue (Math|Vector|VectorDown))
  (bind _returnvalue_2 (Transformation|GetActorRotation))
  (bind _gravityscale (Variables|Default|GetgravityScale))
  (bind _quat (Utilities|RotatortoQuat _returnvalue_2))
  (bind _returnvalue_3 (Class|KismetMathLibrary|QuatRotateVector _quat _returnvalue))
  (bind _returnvalue_4 (* _returnvalue_3 _gravityscale))
  ;[1 1 1] Giving Velocity to Gravity Object
  (for _array_element (Collision|GetOverlappingActors 0 :!class /Script/Engine.Actor)
    (bind _asgravity_object (Utilities|Casting|CastToGravity_Object _array_element))
    (Default|SetCubeGravity _asgravity_object _returnvalue_4))
  (if (Variables|Default|GetAffectCharacter)
    ;[1 1 1] Giving Velocity to Gravity Character
    (for _array_element_2 (Collision|GetOverlappingActors 0 :!class /Script/Engine.Actor)
      (bind _asstage_2character (Utilities|Casting|CastToStage2Character _array_element_2))
      (Transformation|SetActorRotation _asstage_2character (Transformation|GetActorRotation))
      (Physics|AddForce (Variables|/Script/Engine.Character|GetCharacterMovement _asstage_2character) _returnvalue_4)
      (Variables|/Script/Engine.MovementComponent|SetVelocity (Variables|/Script/Engine.Character|GetCharacterMovement _asstage_2character) _returnvalue_4))))

(fn ConstructionScript)