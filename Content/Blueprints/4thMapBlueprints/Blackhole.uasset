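; Black hole hazard that pulls the player character into a deadzone and respawns them.
; Each tick, characters overlapping the Horizontal volume lose gravity, get physics enabled on their capsule and are launched at constant speed toward the Deadzone.
; Leaving that volume turns capsule physics off and resets rotation.
; Entering the Deadzone destroys the actor, then after a short delay spawns and possesses a new character with low gravity at PlayerTransform.
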(event OnComponentBeginOverlap(Deadzone)
  (params (OverlappedComponent :type Primitive%20Component%20Object%20Reference) (OtherActor :type Actor%20Object%20Reference) (OtherComp :type Primitive%20Component%20Object%20Reference) (OtherBodyIndex :type Integer) (bFromSweep :type Boolean) (SweepResult :type Hit%20Result%20Structure%20%28by%20ref%29))
  ;[1 1 1] Destroy and Respawn Character if it is in the blackhole
  (Actor|DestroyActor OtherActor)
  (Utilities|FlowControl|Delay 0.2)
  (bind _returnvalue (Game|SpawnActorfromClass "/Game/ThirdPersonBP/Blueprints/ThirdPersonCharacter.ThirdPersonCharacter_C" (Variables|Default|GetplayerTransform) "Undefined" 0 0))
  (Variables|/Script/Engine.CharacterMovementComponent|SetGravityScale (Variables|/Script/Engine.Character|GetCharacterMovement _returnvalue) 0.3)
  (Pawn|Possess (Game|GetPlayerController 0) _returnvalue))

(event OnComponentEndOverlap(Horizontal)
  (params (OverlappedComponent :type Primitive%20Component%20Object%20Reference) (OtherActor :type Actor%20Object%20Reference) (OtherComp :type Primitive%20Component%20Object%20Reference) (OtherBodyIndex :type Integer))
  ;[1 1 1] Overlapped Event Exception
  (bind _asthird_person_character (Utilities|Casting|CastToThirdPersonCharacter OtherActor))
  (Physics|SetSimulatePhysics (Variables|/Script/Engine.Character|GetCapsuleComponent _asthird_person_character) false)
  (Transformation|SetActorRotation _asthird_person_character "-90.000000, 0, 0"))

(event EventTick
  (params (DeltaSeconds :type Float%20%28single-precision%29))
  ;[1 1 1] Find Overlapped Character
  (for _array_element (Collision|GetOverlappingActors (Variables|Default|GetHorizontal) "/Game/ThirdPersonBP/Blueprints/ThirdPersonCharacter.ThirdPersonCharacter_C" :!class /Script/Engine.PrimitiveComponent)
    (bind _asthird_person_character (Utilities|Casting|CastToThirdPersonCharacter _array_element))
    ;[1 1 1] Stop Character Movement and Set GravityScale 0 before setting velocity
    (Physics|SetEnableGravity (Variables|/Script/Engine.Character|GetCapsuleComponent _asthird_person_character) false)
    (Variables|/Script/Engine.CharacterMovementComponent|SetGravityScale (Variables|/Script/Engine.Character|GetCharacterMovement _asthird_person_character) 0.0)
    (Variables|/Script/Engine.MovementComponent|SetVelocity (Variables|/Script/Engine.Character|GetCharacterMovement _asthird_person_character) "0, 0, 0")
    (Pawn|Components|CharacterMovement|ClearAccumulatedForces (Variables|/Script/Engine.Character|GetCharacterMovement _asthird_person_character))
    ;[1 1 1] Set Velocity
    (Physics|SetSimulatePhysics (Variables|/Script/Engine.Character|GetCapsuleComponent _asthird_person_character) true)
    (Physics|SetPhysicsLinearVelocity (Variables|/Script/Engine.Character|GetCapsuleComponent _asthird_person_character) (* (Math|Vector|GetForwardVector (Math|Rotator|FindLookatRotation (Transformation|GetWorldLocation (Variables|/Script/Engine.Character|GetCapsuleComponent _asthird_person_character)) (Transformation|GetWorldLocation (Variables|Default|GetDeadzone)))) 3e+03) false "None")))

(fn ConstructionScript)