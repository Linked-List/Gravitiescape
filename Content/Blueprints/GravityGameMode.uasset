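; GravityGameMode is a game mode that handles stage streaming, the loading screen and a play timer.
; BeginPlay streams in FirstStage behind a loading widget, then shows a timer widget.
; ChangeStage swaps the timer for the loading screen while it loads the next streamed level and unloads the current one.
; Tick accumulates elapsed minutes and seconds, pausing while IsLoading is set.
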(event EventChangeStage
  (params (CurrentLevel :type Name :default "None") (NextLevel :type Name :default "None"))
  (bind _loadingscreen (Variables|Default|GetLoadingScreen))
  (bind _timer (Variables|Default|GetTimer))
  (Variables|Default|SetisLoading true)
  (Widget|RemovefromParent _timer)
  (UserInterface|Viewport|AddtoViewport _loadingscreen 0)
  (Game|LoadStreamLevel(byName) NextLevel true)
  (Game|UnloadStreamLevel(byName) CurrentLevel false)
  (Widget|RemovefromParent _loadingscreen)
  (UserInterface|Viewport|AddtoViewport _timer 0)
  (Variables|Default|SetisLoading false))

(event EventBeginPlay
  (bind _returnvalue (UserInterface|CreateWidget "/Game/Blueprints/LoadingWidget.LoadingWidget_C"))
  (bind _output_get (Variables|Default|SetLoadingScreen _returnvalue))
  (UserInterface|Viewport|AddtoViewport _output_get 0)
  (Game|LoadStreamLevel(byName) "FirstStage" true)
  (bind _returnvalue_2 (UserInterface|CreateWidget "/Game/Blueprints/TimerWidget.TimerWidget_C"))
  (Variables|Default|SetTimer _returnvalue_2)
  (Widget|RemovefromParent _output_get)
  (UserInterface|Viewport|AddtoViewport _returnvalue_2 0)
  (Variables|Default|SetisLoading false))

(event EventTick
  (params (DeltaSeconds :type Float%20%28single-precision%29))
  (if (not (Variables|Default|GetisLoading))
    (if (>= (+ DeltaSeconds (Variables|Default|GetTimerSec)) 6e+01)
      (Variables|Default|SetTimerSec (- (+ DeltaSeconds (Variables|Default|GetTimerSec)) 6e+01))
      (Variables|Default|SetTimerMin (+ (Variables|Default|GetTimerMin) 1))
      (else
        (Variables|Default|SetTimerSec (+ DeltaSeconds (Variables|Default|GetTimerSec)))))))

(fn ConstructionScript)